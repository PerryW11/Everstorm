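; BP_AidoSecondary is an actor, apparently Aido's secondary attack, that explodes on contact.
; On overlap it casts player 0's character to BP_Aido and ignores that character, doing nothing if the cast fails.
; Any other overlap sets a one-shot Hit flag, spawns BP_Explosion at the actor's location and destroys the actor.
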(event `self.ReceiveBeginPlay`)

(event `self.ReceiveActorBeginOverlap`
  (params (OtherActor :type "Actor Object Reference"))
  (bind _asbp_aido (cast `/Game/Aido/Blueprints/BP_Aido` (`GameplayStatics.GetPlayerCharacter` 0)))
  (if (== OtherActor _asbp_aido)
    _
    (elif (not (`self.Hit`))
      (set `self.Hit` true)
      (`|SpawnActorFromClass` "/Game/Aido/Blueprints/BP_Explosion.BP_Explosion_C" (`KismetMathLibrary.MakeTransform` (`self.K2_GetActorLocation`)) "Undefined" "OverrideRootScale" null null)
      (`self.K2_DestroyActor`))))

(fn `UserConstructionScript`)