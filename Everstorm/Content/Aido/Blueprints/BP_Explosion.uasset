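; BP_Explosion is a short-lived explosion actor that kills zombies and hurts the player.
; On BeginPlay it plays a sound at the world origin, fires its ForceComponent impulse, then destroys itself after a brief delay.
; Overlapping live BP_ZombieAI actors die, ragdoll and trigger a KillPopup widget.
; An overlapping BP_Aido takes damage through stacked fixed-amount TakeDamage calls and gets a DamageEffect widget.
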(event `self.ReceiveBeginPlay`
  (`GameplayStatics.PlaySoundAtLocation` "/Game/StarterContent/Audio/Explosion01.Explosion01" (0.0 0.0 0.0) (struct) 0.4 1.0 0.0 null null null)
  (`RadialForceComponent.FireImpulse` (`self.ForceComponent`))
  (`KismetSystemLibrary.Delay` 0.8)
  (`self.K2_DestroyActor`))

(event `self.ReceiveActorBeginOverlap`
  (params (OtherActor :type "Actor Object Reference"))
  (`|ExecutionSequence`
    (:`then_0`
      (bind _asbp_zombie_ai (cast `/Game/EnemyAI/BP_ZombieAI` OtherActor))
      (if (not (`/Game/EnemyAI/BP_ZombieAI.IsDead` _asbp_zombie_ai))
        (set `/Game/EnemyAI/BP_ZombieAI.EnemyHealth` 0.0 _asbp_zombie_ai)
        (set `/Game/EnemyAI/BP_ZombieAI.IsDead` true _asbp_zombie_ai)
        (`PrimitiveComponent.SetSimulatePhysics` (`Character.Mesh` _asbp_zombie_ai) true)
        (bind _returnvalue (`|CreateWidget` "/Game/Aido/Blueprints/KillPopup.KillPopup_C"))
        (`UserWidget.AddToViewport` _returnvalue 0)))
    (:`then_1`
      (bind _asbp_aido (cast `/Game/Aido/Blueprints/BP_Aido` OtherActor))
      (`/Game/Aido/Blueprints/BP_Aido.TakeDamage20%` _asbp_aido)
      (`/Game/Aido/Blueprints/BP_Aido.TakeDamage20%` _asbp_aido)
      (`/Game/Aido/Blueprints/BP_Aido.TakeDamage10%` _asbp_aido)
      (bind _returnvalue_2 (`|CreateWidget` "/Game/Aido/Blueprints/DamageEffect.DamageEffect_C"))
      (`UserWidget.AddToViewport` _returnvalue_2 0))))

(fn `UserConstructionScript`)