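; BP_Explosion is a short-lived explosion actor that kills zombies caught in it.
; On BeginPlay it fires an impulse from its force component, then destroys itself after a brief delay.
; Any living BP_ZombieAI overlapping it has its health zeroed, is flagged dead, ragdolls through mesh physics, and spawns a KillPopup widget on screen.
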(event `self.ReceiveBeginPlay`
  (`RadialForceComponent.FireImpulse` (`self.ForceComponent`))
  (`KismetSystemLibrary.Delay` 0.8)
  (`self.K2_DestroyActor`))

(event `self.ReceiveActorBeginOverlap`
  (params (OtherActor :type "Actor Object Reference"))
  (bind _asbp_zombie_ai (cast `/Game/EnemyAI/BP_ZombieAI` OtherActor))
  (if (not (`/Game/EnemyAI/BP_ZombieAI.IsDead` _asbp_zombie_ai))
    (set `/Game/EnemyAI/BP_ZombieAI.EnemyHealth` 0.0 _asbp_zombie_ai)
    (set `/Game/EnemyAI/BP_ZombieAI.IsDead` true _asbp_zombie_ai)
    (`PrimitiveComponent.SetSimulatePhysics` (`Character.Mesh` _asbp_zombie_ai) true)
    (bind _returnvalue (`|CreateWidget` "/Game/LordAido/Blueprints/KillPopup.KillPopup_C"))
    (`UserWidget.AddToViewport` _returnvalue 0)))

(fn `UserConstructionScript`)